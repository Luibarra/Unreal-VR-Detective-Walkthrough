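; BP_Cup is a cup actor that can be picked up and released, with a proximity pop-up widget.
; Its Interact event attaches it to the hand with physics off and hides the pop-up, then reverses this on release.
; The trigger box calls the widget's show and hide functions as the player pawn enters and leaves.
; While visible, the pop-up turns each Tick on yaw only, based on camera position.
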(event OnComponentBeginOverlap(TriggerBox)
  (params (OverlappedComponent :type Primitive%20Component%20Object%20Reference) (OtherActor :type Actor%20Object%20Reference) (OtherComp :type Primitive%20Component%20Object%20Reference) (OtherBodyIndex :type Integer) (bFromSweep :type Boolean) (SweepResult :type Hit%20Result%20Structure%20%28by%20ref%29))
  ;[1 1 1] UI Prox Anim
  (if (== OtherActor (Game|Player|GetPlayerPawn 0))
    (bind _aspop_up_ui (Utilities|Casting|CastToPopUpUI (UserInterface|GetUserWidgetObject (Variables|Default|GetPopUpUI))))
    (Default|CallShowPopUp _aspop_up_ui)))

(event OnComponentEndOverlap(TriggerBox)
  (params (OverlappedComponent :type Primitive%20Component%20Object%20Reference) (OtherActor :type Actor%20Object%20Reference) (OtherComp :type Primitive%20Component%20Object%20Reference) (OtherBodyIndex :type Integer))
  ;[1 1 1] UI Prox Anim
  (if (== OtherActor (Game|Player|GetPlayerPawn 0))
    (bind _aspop_up_ui (Utilities|Casting|CastToPopUpUI (UserInterface|GetUserWidgetObject (Variables|Default|GetPopUpUI))))
    (Default|CallHidePopUp _aspop_up_ui)))

(event EventInteract
  (params (Hand :type Scene%20Component%20Object%20Reference) (isHolding :type Boolean))
  ;[1 1 1] Held
  (if isHolding
    (Physics|SetSimulatePhysics (Variables|Default|GetStaticMesh) false)
    (Transformation|AttachComponentToComponent Hand "None" "KeepWorld" "KeepWorld" "KeepWorld" true)
    (Rendering|SetVisibility (Variables|Default|GetPopUpUI) false false)
    (else
      (Transformation|DetachFromActor "KeepWorld" "KeepWorld" "KeepWorld")
      (Physics|SetSimulatePhysics (Variables|Default|GetStaticMesh) true)
      (Rendering|SetVisibility (Variables|Default|GetPopUpUI) true false))))

(event EventTick
  (params (DeltaSeconds :type Float%20%28single-precision%29))
  ;[1 1 1] Faces Player Function each Tick
  (if (Variables|/Script/Engine.SceneComponent|GetbVisible (Variables|Default|GetPopUpUI))
    (CallFunction|UpdatePopUpFacing)))

(fn ConstructionScript)

(fn UpdatePopUpFacing
  (Transformation|SetWorldRotation (Variables|Default|GetPopUpUI) (Math|Rotator|MakeRotator 0.0 0.0 (.yaw (Math|Rotator|FindLookatRotation (Camera|GetCameraLocation (Game|GetPlayerCameraManager 0)) (Transformation|GetWorldLocation (Variables|Default|GetPopUpUI))))) false false))